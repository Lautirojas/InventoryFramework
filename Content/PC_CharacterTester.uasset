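; Player controller for a test character that manages the player and chest inventory UI.
; For the local player, it adds input mappings and creates the main HUD from the pawn's InventoryComponent; chest data is supplied separately.
; Toggle events show or collapse each panel, with the cursor shown while either is open.
; Drag-and-drop transfer requests route through a server request event that calls TransferItemTo on the source inventory, supporting multiplayer.
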(event `self.ReceiveBeginPlay`
  ;[0.1406 0.1406 0.1406 0.5] Only add input mappings to local players
  (if (`self.IsLocalPlayerController`)
    ;[0.1406 0.1406 0.1406 0.5] Add regular input mappings
    (`EnhancedInputSubsystemInterface.AddMappingContext` (subsystem `EnhancedInputLocalPlayerSubsystem`) "/Game/Input/IMC_Default.IMC_Default" 0 (struct))
    (`EnhancedInputSubsystemInterface.AddMappingContext` (subsystem `EnhancedInputLocalPlayerSubsystem`) "/Game/Input/IMC_MouseLook.IMC_MouseLook" 0 (struct))
    ; Get Component
    (bind _ascharacter (cast `Character` (`self.K2_GetPawn`)))
    ;[0.1406 0.1406 0.1406 0.5] Create Main Widget
    (`KismetSystemLibrary.DelayUntilNextTick`)
    (bind _returnvalue (`self.GetComponentByClass` _ascharacter "/Script/InventoryFramework.InventoryComponent"))
    (bind _returnvalue_2 (`|CreateWidget` "/Game/HUD/UW_Main.UW_Main_C" self _returnvalue))
    (bind _uw_inventorygrid (`/Game/HUD/UW_InventoryPanel.UW_InventoryGrid` (`/Game/HUD/UW_Main.UW_PlayerInventory` _returnvalue_2)))
    (`InventoryGridWidget.SetInventoryData` _uw_inventorygrid _returnvalue)
    (`UserWidget.AddToViewport` _returnvalue_2 0)
    (set `self.MainHUD` _returnvalue_2)
    (add `InventoryGridWidget.OnInventoryTransferRequested` _uw_inventorygrid (`|CreateDelegate` :!event `HandleInventoryTransferRequest`))))

(event `/Game/Blueprints/BPI_Hud.ToggleInventory`
  ; Toggle Inventory
  (bind _mainhud (`self.MainHUD`)
    (:`then`
      (bind _uw_playerinventory (`/Game/HUD/UW_Main.UW_PlayerInventory` _mainhud))
      (switch `ESlateVisibility` (`Widget.Visibility` _uw_playerinventory)
        (:`Visible`
          (`Widget.SetVisibility` _uw_playerinventory "Collapsed"))
        (:`Collapsed`
          (`Widget.SetVisibility` _uw_playerinventory "Visible")))
      (`self.NeedCursor`))
    (:`else`)))

(event `/Game/Blueprints/BPI_Hud.SetInitalInventoryChest`
  (params (InventoryRef :type "InventoryComponent Object Reference"))
  ; Get Chest Component
  (bind _mainhud (`self.MainHUD`)
    (:`then`
      (bind _uw_inventorygrid (`/Game/HUD/UW_InventoryPanel.UW_InventoryGrid` (`/Game/HUD/UW_Main.UW_ChestInventory` _mainhud)))
      (`InventoryGridWidget.SetInventoryData` _uw_inventorygrid InventoryRef)
      (add `InventoryGridWidget.OnInventoryTransferRequested` _uw_inventorygrid (`|CreateDelegate` :!event `HandleInventoryTransferRequest`)))
    (:`else`)))

(event `HandleInventoryTransferRequest`
  (params (SourceInventory :type "InventoryComponent Object Reference") (TargetInventory :type "InventoryComponent Object Reference") (SourceIndex :type Integer) (TargetIndex :type Integer))
  ; Handle Multiplayer Drag/Drop
  (`self.Server_RequestInventoryTransfer` SourceInventory TargetInventory SourceIndex TargetIndex))

(event `/Game/Blueprints/BPI_Hud.ToggleChestInventory`
  ; Toggle Chest Inventory visiblity
  (bind _mainhud (`self.MainHUD`)
    (:`then`
      (bind _uw_chestinventory (`/Game/HUD/UW_Main.UW_ChestInventory` _mainhud))
      (switch `ESlateVisibility` (`Widget.Visibility` _uw_chestinventory)
        (:`Visible`
          (`Widget.SetVisibility` _uw_chestinventory "Collapsed"))
        (:`Collapsed`
          (`Widget.SetVisibility` _uw_chestinventory "Visible")))
      (`self.NeedCursor`))
    (:`else`)))

(event `Server_RequestInventoryTransfer`
  (params (SourceInventory :type "InventoryComponent Object Reference") (TargetInventory :type "InventoryComponent Object Reference") (SourceIndex :type Integer) (TargetIndex :type Integer))
  ; Handle Multiplayer Drag/Drop
  (`InventoryComponent.TransferItemTo` SourceInventory TargetInventory SourceIndex TargetIndex))

(fn `GetPCRef`
  (returns (`PC Ref` :type "/Game/PC_CharacterTester Object Reference"))
  (return self))

(fn `NeedCursor`
  (bind _mainhud (`self.MainHUD`)
    (:`then`
      (if (or (`|EnumEquality` (`Widget.GetVisibility` (`/Game/HUD/UW_Main.UW_ChestInventory` _mainhud)) "Visible") (`|EnumEquality` (`Widget.GetVisibility` (`/Game/HUD/UW_Main.UW_PlayerInventory` _mainhud)) "Visible"))
        (set `self.bShowMouseCursor` true)
        (else
          (set `self.bShowMouseCursor` false))))
    (:`else`)))

(fn `UserConstructionScript`)